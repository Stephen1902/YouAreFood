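; BP_Fairy is a world item actor showing an animated fairy with randomized colours.
; On BeginPlay it creates a dynamic material from M_FairyBody and picks body and hair colours from one palette and flesh colour from another.
; After a random delay of up to a second it loops the fairy animation, so multiple fairies do not animate in sync.
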(event `self.ReceiveBeginPlay`
  (bind _returnvalue (`PrimitiveComponent.CreateDynamicMaterialInstance` (`self.SkeletalMesh`) 0 "/Game/Materials/M_FairyBody.M_FairyBody" "None"))
  (`MaterialInstanceDynamic.SetVectorParameterValue` _returnvalue "BodyColour" (`KismetArrayLibrary.Array_Random` (`self.BodyColours`)))
  (`MaterialInstanceDynamic.SetVectorParameterValue` _returnvalue "FleshColour" (`KismetArrayLibrary.Array_Random` (`self.FleshColours`)))
  (`MaterialInstanceDynamic.SetVectorParameterValue` _returnvalue "HairColour" (`KismetArrayLibrary.Array_Random` (`self.BodyColours`)))
  (`KismetSystemLibrary.Delay` (`KismetMathLibrary.RandomFloatInRange` 0.0 1.0))
  (`SkeletalMeshComponent.PlayAnimation` (`self.SkeletalMesh`) "/Game/Meshes/Level/FairyBase2_Anim.FairyBase2_Anim" true))

(fn `UserConstructionScript`)