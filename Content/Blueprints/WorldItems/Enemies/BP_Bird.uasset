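; BP_Bird is a bird world item, filed under enemies, that reacts when triggered by an overlap.
; On BeginPlay it randomly picks a blackbird or sparrow material for its skeletal mesh.
; Its OverlapTriggered event, whose caller is not in this graph, plays a one-shot bird animation, sets the mesh's relative scale and plays a pitched-up 2D caught sound.
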(event `self.ReceiveBeginPlay`
  (if (`KismetMathLibrary.RandomBool`)
    (`PrimitiveComponent.SetMaterial` (`self.SkeletalMeshComp`) 0 "/Game/Meshes/Enemies/Bird/M_Blackbird.M_Blackbird")
    (else
      (`PrimitiveComponent.SetMaterial` (`self.SkeletalMeshComp`) 0 "/Game/Meshes/Enemies/Bird/M_Sparrow.M_Sparrow"))))

(event `self.OverlapTriggered`
  (`SkeletalMeshComponent.PlayAnimation` (`self.SkeletalMeshComp`) "/Game/Meshes/Enemies/Bird/Animations/Bird_Anim.Bird_Anim" false)
  (`SceneComponent.SetRelativeScale3D` (`self.SkeletalMeshComp`) (100.0 100.0 100.0))
  (`GameplayStatics.PlaySound2D` "/Game/Blueprints/Sounds/bird_caught.bird_caught" 1.0 1.5 0.0 null null false))

(fn `UserConstructionScript`)